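; BP_FireLight is a farm house actor that flickers a point light to imitate firelight.
; A Timeline started at BeginPlay uses its update as a tick, lerping the light's intensity most of the way toward a target value on every update.
; A short randomized Delay on the same update throttles how often that target is re-rolled within a fixed range, giving an irregular but softened flicker.
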(event EventBeginPlay
  (bind _pointlight (Variables|Default|GetPointLight))
  (Timeline|Timeline Play
    (:Update
      (Utilities|FlowControl|Sequence
        (:then_0
          (Rendering|Components|Light|SetIntensity _pointlight (Math|Float|Lerp (Variables|/Script/Engine.LightComponentBase|GetIntensity _pointlight) (Variables|Default|GetLightIntencityFloat) 0.8)))
        (:then_1
          (Utilities|FlowControl|Delay (Math|Random|RandomFloatinRange 0.08 0.1))
          (Variables|Default|SetLightIntencityFloat (Math|Random|RandomFloatinRange 2.5e+03 3e+03)))))))

(event Collision|EventActorBeginOverlap
  (params (OtherActor :type Actor%20Object%20Reference)))

(event EventTick
  (params (DeltaSeconds :type Float%20%28single-precision%29)))

(fn ConstructionScript)